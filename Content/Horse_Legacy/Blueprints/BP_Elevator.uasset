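; Elevator actor that moves vertically by a Direction offset when something overlaps its Box trigger, with no filter on the overlapping actor.
; A FlipFlop alternates each overlap between playing and reversing a timeline, whose track lerps the actor's location along Z.
; StartLocation is re-captured on every overlap, so the reverse run is relative to the current position rather than the original one.
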(event `self.Box.OnComponentBeginOverlap`
  (params (OverlappedComponent :type "PrimitiveComponent Object Reference") (OtherActor :type "Actor Object Reference") (OtherComp :type "PrimitiveComponent Object Reference") (OtherBodyIndex :type Integer) (bFromSweep :type Boolean) (SweepResult :type "HitResult Structure (by ref)"))
  (bind _startlocation (`self.StartLocation`))
  (set `self.StartLocation` (`self.K2_GetActorLocation`))
  (`/Engine/EditorBlueprintResources/StandardMacros.FlipFlop`
    (:`A`
      (bind (_direction _newtrack_0) (`Timeline|Timeline_0` :!label _label)
        (:`Update`
          (`self.K2_SetActorLocation` (`KismetMathLibrary.VLerp` _startlocation (`KismetMathLibrary.MakeVector` (.x _startlocation) (.y _startlocation) (+ (.z _startlocation) (`self.Direction`))) _newtrack_0)))))
    (:`B`
      (goto _label :!via `Reverse`))))

(fn `UserConstructionScript`)