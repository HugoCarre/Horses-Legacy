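; Flying arrow projectile that sticks into skeletal targets by swapping itself for a fixed arrow actor.
; Its first overlap, gated to run once, fires a short forward capsule trace from the Sphere on Visibility.
; If the hit names a bone, it stops, moves to the impact point, spawns BP_ArrowFix attached to that bone and destroys itself.
; Otherwise it stays in place as a projectile and ignores later overlaps.
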(event `self.ReceiveActorBeginOverlap`
  (params (OtherActor :type "Actor Object Reference"))
  (bind _sphere (`self.Sphere`))
  (bind _returnvalue (`SceneComponent.K2_GetComponentLocation` _sphere))
  (if (`self.DoOnce`)
    (set `self.DoOnce` false)
    (bind (_outhit _returnvalue_2) (`KismetSystemLibrary.CapsuleTraceSingle` _returnvalue (+ _returnvalue (* (`KismetMathLibrary.GetForwardVector` (`SceneComponent.K2_GetComponentRotation` _sphere)) 200.0)) 0.0 0.0 "TraceTypeQuery1" false (`|MakeArray` null :!type "Actor Object Reference")))
    (if _returnvalue_2
      (bind (_bblockinghit _binitialoverlap _time _distance _location _impactpoint _normal _impactnormal _physmat _hitactor _hitcomponent _hitbonename) (`GameplayStatics.BreakHitResult` _outhit))
      (if (not (== _hitbonename "None"))
        (`MovementComponent.StopMovementImmediately` (`self.ProjectileMovement`))
        (`self.K2_SetActorLocation` _impactpoint)
        (bind _returnvalue_3 (`|SpawnActorFromClass` "/Game/Horse_Legacy/Blueprints/BP_ArrowFix.BP_ArrowFix_C" (`self.GetTransform` self) "Undefined" "OverrideRootScale" null null))
        (`SceneComponent.K2_AttachToComponent` (`/Game/Horse_Legacy/Blueprints/BP_ArrowFix.Sphere` _returnvalue_3) _hitcomponent _hitbonename "KeepWorld" "KeepWorld" "KeepWorld" true)
        (`self.K2_DestroyActor`)))))

(fn `UserConstructionScript`)