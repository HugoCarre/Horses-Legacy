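; Rideable horse pawn with rein-and-leg controls, mount/dismount swapping possession with ThirdPersonCharacter, and charged arrow shooting.
; Timed counts of simultaneous leg presses raise the gait, add acceleration bonuses or trigger rearing; gaits decay over time.
; Tick eases speed toward per-gait map values, moves the actor manually, handles sidepasses and aligns it to ground normals.
; Reins turn or stop the horse; jumping requires a straight gallop.
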(event `InputAxis|LookUp`
  (params (AxisValue :type "Float (single-precision)"))
  ;[1 1 1] LookUp  camera
  (if (`self.IsMounting`)
    (`SceneComponent.K2_SetWorldRotation` (`self.SpringArm`) (`KismetMathLibrary.MakeRotator` (.roll (`SceneComponent.K2_GetComponentRotation` (`self.SpringArm`))) (`KismetMathLibrary.ClampAngle` (+ (* AxisValue (`self.DeltaTime`) (`self.CameraSpeed`)) (.pitch (`SceneComponent.K2_GetComponentRotation` (`self.SpringArm`)))) 300.0 85.0) (.yaw (`SceneComponent.K2_GetComponentRotation` (`self.SpringArm`)))) false false)))

(event `OnBothLegsTriggered_Event`
  ;[1 1 1] Custom Events
  ;;[1 1 1] Increase nB pressure done  LT + RT
  (set `self.NbBothLegsTriggered` (+ (`self.NbBothLegsTriggered`) 1)))

(event `CustomEvent_0` :!signature `self.OnMoveStateChanged`
  (params (MoveState :type "/Game/Horse_Legacy/Blueprints/ENUM_HorseMoveState Enum" :default "NewEnumerator0"))
  ;[1 1 1] Custom Events
  (set `self.ElapsedStateDurationTime` 0.0))

(event `OnDirectionChange_Event` :!signature `self.OnDirectionChanged`
  (params (InputValue :type "Float (double-precision)"))
  ;[1 1 1] Custom Events
  (set `self.IsRotating` (not (`KismetMathLibrary.NearlyEqual_FloatFloat` InputValue))))

(event `InputAxis|Turn`
  (params (AxisValue :type "Float (single-precision)"))
  ;[1 1 1] Turn camera
  (if (`self.IsMounting`)
    (`SceneComponent.K2_SetWorldRotation` (`self.SpringArm`) (`KismetMathLibrary.MakeRotator` (.roll (`SceneComponent.K2_GetComponentRotation` (`self.SpringArm`))) (.pitch (`SceneComponent.K2_GetComponentRotation` (`self.SpringArm`))) (+ (* AxisValue (`self.DeltaTime`) (`self.CameraSpeed`)) (.yaw (`SceneComponent.K2_GetComponentRotation` (`self.SpringArm`))))) false false)))

(event `self.ReceiveBeginPlay`
  ;[1 1 1] Custom Events
  (`|ExecutionSequence`
    (:`then_0`
      (add `self.OnBothLegsTriggered` (delegate `OnBothLegsTriggered_Event`))
      (add `self.OnMoveStateChanged` (delegate `CustomEvent_0`))
      (add `self.OnDirectionChanged` (delegate `OnDirectionChange_Event`)))))

(event `self.ReceiveTick`
  (params (DeltaSeconds :type "Float (single-precision)"))
  (bind _value (`self.GetCurrentMaxSpeed`))
  (bind _value_2 (`self.GetCurrentMaxSpeed`))
  (bind _returnvalue (`SceneComponent.K2_GetComponentLocation` (`self.CapsuleComponent`)))
  (set `self.DeltaTime` DeltaSeconds)
  (if (`self.IsMounting`)
    (`|ExecutionSequence`
      (:`then_0`
        (`self.UpdateBothLegsTimer`))
      (:`then_1`
        ;[1 1 1] Handle Horse current Speed
        (if (< (`self.CurrentSpeed`) (`self.GetCurrentMaxSpeed`))
          ;;[1 1 1] Have to increase current speed (ACCELERATE)
          (set `self.IsAccelerating` true)
          (`self.SetCurrentSpeed` (+ (`self.CurrentSpeed`) (* (+ (`self.Get Current Acceleration`) (* (`self.NbAccelerationBonus`) (`self.AccelerationBonusValue`))) (`self.DeltaTime`))))
          (if (>= (`self.CurrentSpeed`) _value)
            (`self.SetCurrentSpeed` _value)
            (`KismetSystemLibrary.PrintString` (`KismetStringLibrary.Conv_DoubleToString` (`self.NbAccelerationBonus`)))
            (set `self.NbAccelerationBonus` 0.0)
            (set `self.IsAccelerating` false))
          (else
            ;;[1 1 1] Have to decrease current speed (DECELERATE)
            (set `self.IsAccelerating` false)
            (set `self.NbAccelerationBonus` 0.0)
            (if (> (`self.CurrentSpeed`) (`self.GetCurrentMaxSpeed`))
              (`self.SetCurrentSpeed` (- (`self.CurrentSpeed`) (* (`self.DecelerateSpeed`) (`self.DeltaTime`))))
              (if (<= (`self.CurrentSpeed`) _value_2)
                (`self.SetCurrentSpeed` _value_2))))))
      (:`then_2`
        ;[1 1 1] Horse Motor movement
        (if (not (or (`self.IsSpecialMoving`) (`self.IsRearing`)))
          (`self.K2_SetActorLocation` (+ (* (`self.GetActorForwardVector`) (* (`self.CurrentSpeed`) (`self.DeltaTime`))) (`self.K2_GetActorLocation`)))))
      (:`then_3`
        (if (or (not (`NavMovementComponent.IsFalling` (`self.CharacterMovement`))) (not (`self.IsRearing`)))
          ;[1 1 1] Right sidepass
          (if (and (`self.IsLegSpecialLeftTriggered`) (`self.IsRightLegTrigger`))
            (if (not (`self.IsSpecialMoving`))
              (set `self.StateBeforeSpecaialMove` (`self.MovementState`)))
            (bind _output_get (set `self.MovementState` "NewEnumerator1"))
            (`self.OnMoveStateChanged` _output_get)
            (set `self.IsSpecialMoving` true)
            (set `self.NbBothLegsTriggered` 0)
            (set `self.DecelerateSpeed` (/ (`self.CurrentSpeed`) (`self.DecelarateDelay`)))
            (`self.K2_SetActorLocation` (+ (* (`self.GetActorRightVector`) (* (`self.SidePassSpeed`) (`self.DeltaTime`))) (`self.K2_GetActorLocation`)))
            (else
              ;[1 1 1] Left sidepass
              (if (and (`self.IsLegSpecialRightTriggered`) (`self.IsLeftLegTrigger`))
                (if (not (`self.IsSpecialMoving`))
                  (set `self.StateBeforeSpecaialMove` (`self.MovementState`)))
                (bind _output_get_2 (set `self.MovementState` "NewEnumerator1"))
                (`self.OnMoveStateChanged` _output_get_2)
                (set `self.IsSpecialMoving` true)
                (set `self.NbBothLegsTriggered` 0)
                (set `self.DecelerateSpeed` (/ (`self.CurrentSpeed`) (`self.DecelarateDelay`)))
                (`self.K2_SetActorLocation` (+ (* (* (`self.GetActorRightVector`) -1.0) (* (`self.SidePassSpeed`) (`self.DeltaTime`))) (`self.K2_GetActorLocation`)))
                (elif (`self.IsSpecialMoving`)
                  (bind _output_get_3 (set `self.MovementState` (`self.StateBeforeSpecaialMove`)))
                  (`self.OnMoveStateChanged` _output_get_3)
                  (set `self.DecelerateSpeed` (/ (`self.CurrentSpeed`) (`self.DecelarateDelay`)))
                  (set `self.IsSpecialMoving` false)
                  (set `self.NbBothLegsTriggered` 0)))))))
      (:`then_4`
        (if (`self.HasToRear`)
          (set `self.HasToRear` false)
          (set `self.IsRearing` true)
          (bind _output_get_4 (set `self.MovementState` "NewEnumerator0"))
          (`self.OnMoveStateChanged` _output_get_4)
          (set `self.DecelerateSpeed` (/ (`self.CurrentSpeed`) (`self.DecelarateDelay`)))
          (set `self.NbBothLegsTriggered` 0)
          (bind (_direction _rearing) (`Timeline|Timeline_0` :!via `PlayFromStart`)
            (:`Update`
              (`self.K2_SetActorRotation` (`KismetMathLibrary.MakeRotator` (.roll (`self.K2_GetActorRotation`)) (`KismetMathLibrary.Lerp` 0.0 30.0 _rearing) (.yaw (`self.K2_GetActorRotation`)))))
            (:`Finished`
              (set `self.IsRearing` false)))))
      (:`then_5`
        (if (not (or (`NavMovementComponent.IsFalling` (`self.CharacterMovement`)) (`self.IsRearing`)))
          (bind _outhit (`KismetSystemLibrary.LineTraceSingle` _returnvalue (+ _returnvalue (0.0 0.0 -100.0)) "TraceTypeQuery1"))
          (`self.K2_SetActorRotation` (`KismetMathLibrary.MakeRotator` (.roll (`KismetMathLibrary.MakeRotFromZX` (`.ImpactNormal` (`GameplayStatics.BreakHitResult` _outhit)) (`self.GetActorForwardVector`))) (.pitch (`KismetMathLibrary.MakeRotFromZX` (`.ImpactNormal` (`GameplayStatics.BreakHitResult` _outhit)) (`self.GetActorForwardVector`))) (.yaw (`self.K2_GetActorRotation`)))))))))

(event `InputAction|LegL`
  (params (Key :type "Key Structure"))
  ;[1 1 1] Legs Trigger ( pas / trot /galop)
  (:`Pressed`
    (bind _isa (`/Engine/EditorBlueprintResources/StandardMacros.FlipFlop` :!label _label)
      (:`A`
        _)
      (:`B`
        _))
    (set `self.IsLeftLegTrigger` _isa)
    (if (not (or (`self.IsLegSpecialLeftTriggered`) (`self.IsLegSpecialRightTriggered`) (`self.IsRearing`) (not (`self.IsMounting`))))
      (bind _result (`self.AreBothLegsTriggered`))
      (if _result
        (`self.OnBothLegsTriggered` :!label _label_2))))
  (:`Released`
    (goto _label)))

(event `InputAction|LegR`
  (params (Key :type "Key Structure"))
  ;[1 1 1] Legs Trigger ( pas / trot /galop)
  (:`Pressed`
    (bind _isa (`/Engine/EditorBlueprintResources/StandardMacros.FlipFlop` :!label _label_3)
      (:`A`
        _)
      (:`B`
        _))
    (set `self.IsRightLegTrigger` _isa)
    (if (not (or (`self.IsLegSpecialLeftTriggered`) (`self.IsLegSpecialRightTriggered`) (`self.IsRearing`) (not (`self.IsMounting`))))
      (bind _result (`self.AreBothLegsTriggered`))
      (if _result
        (goto _label_2))))
  (:`Released`
    (goto _label_3)))

(event `InputAxis|Stop`
  (params (AxisValue :type "Float (single-precision)"))
  ;[1 1 1] Rein back (stop the mounture)
  (if (`NavMovementComponent.IsFalling` (`self.CharacterMovement`))
    _
    (elif (<= AxisValue -1.0)
      (bind _output_get (set `self.MovementState` "NewEnumerator0"))
      (set `self.DecelerateSpeed` (/ (`self.CurrentSpeed`) (`self.DecelarateDelay`)))
      (`self.OnMoveStateChanged` _output_get)
      (set `self.NbBothLegsTriggered` 0))))

(event `InputAxis|MoveRight`
  (params (AxisValue :type "Float (single-precision)"))
  ;[1 1 1] Rein direction (Horse Rotation)
  (if (not (`self.IsSpecialMoving`))
    (`self.OnDirectionChanged` AxisValue)
    (`self.K2_SetActorRotation` (`KismetMathLibrary.MakeRotator` (.roll (`self.K2_GetActorRotation`)) (.pitch (`self.K2_GetActorRotation`)) (+ (* AxisValue (`self.DeltaTime`) (`self.GetCurrentTurnSpeed`)) (.yaw (`self.K2_GetActorRotation`)))))))

(event `InputAction|Jump`
  (params (Key :type "Key Structure"))
  (bind _returnvalue (and (`|EnumEquality` (`self.MovementState`) "NewEnumerator3") (not (`self.IsRotating`)) (`self.IsMounting`)))
  (:`Pressed`
    (if _returnvalue
      (`self.Jump`)
      (`self.K2_SetActorRotation` (`KismetMathLibrary.RInterpTo` (`self.K2_GetActorRotation`) (struct) (`self.DeltaTime`) 0.5))))
  (:`Released`
    (if _returnvalue
      (`self.StopJumping`))))

(event `InputAction|LegSpecialLeft`
  (params (Key :type "Key Structure"))
  (:`Pressed`
    (bind _isa (`/Engine/EditorBlueprintResources/StandardMacros.FlipFlop` :!label _label_4)
      (:`A`
        _)
      (:`B`
        _))
    (set `self.IsLegSpecialLeftTriggered` _isa))
  (:`Released`
    (goto _label_4)))

(event `InputAction|LegSpecialRight`
  (params (Key :type "Key Structure"))
  (:`Pressed`
    (bind _isa (`/Engine/EditorBlueprintResources/StandardMacros.FlipFlop` :!label _label_5)
      (:`A`
        _)
      (:`B`
        _))
    (set `self.IsLegSpecialRightTriggered` _isa))
  (:`Released`
    (goto _label_5)))

(event `self.TriggerZone.OnComponentBeginOverlap`
  (params (OverlappedComponent :type "PrimitiveComponent Object Reference") (OtherActor :type "Actor Object Reference") (OtherComp :type "PrimitiveComponent Object Reference") (OtherBodyIndex :type Integer) (bFromSweep :type Boolean) (SweepResult :type "HitResult Structure (by ref)"))
  (set `self.HorseMan` (cast `/Game/ThirdPersonBP/Blueprints/ThirdPersonCharacter` OtherActor :!pure true)))

(event `self.TriggerZone.OnComponentEndOverlap`
  (params (OverlappedComponent :type "PrimitiveComponent Object Reference") (OtherActor :type "Actor Object Reference") (OtherComp :type "PrimitiveComponent Object Reference") (OtherBodyIndex :type Integer))
  (set `self.HorseMan` null))

(event `self.ReceivePossessed`
  (params (NewController :type "Controller Object Reference"))
  (`KismetSystemLibrary.PrintString` "Horse"))

(event `InputAction|SwitchCharac`
  (params (Key :type "Key Structure"))
  (bind _returnvalue (`GameplayStatics.GetPlayerController` 0))
  (bind _returnvalue_2 (`GameplayStatics.GetPlayerController` 0))
  (:`Pressed`
    (if (`self.IsMounting`)
      (`SceneComponent.SetHiddenInGame` (`self.StaticMesh`) true true)
      (bind _returnvalue_3 (`|SpawnActorFromClass` "/Game/ThirdPersonBP/Blueprints/ThirdPersonCharacter.ThirdPersonCharacter_C" (`KismetMathLibrary.MakeTransform` (+ (`self.K2_GetActorLocation`) (0.0 50.0 0.0))) "Undefined" "OverrideRootScale" null null))
      (`Controller.UnPossess` _returnvalue)
      (`Controller.Possess` _returnvalue _returnvalue_3)
      (set `self.IsMounting` false)
      (else
        (`self.K2_DestroyActor` (`self.HorseMan`))
        (`SceneComponent.SetHiddenInGame` (`self.StaticMesh`) false true)
        (`Controller.UnPossess` _returnvalue_2)
        (`Controller.Possess` _returnvalue_2 self)
        (set `self.IsMounting` true)))))

(event `InputAction|Fire`
  (params (Key :type "Key Structure"))
  (bind _arrowmaxspeed (`self.ArrowMaxSpeed`))
  ;[1 1 1] shoot
  (:`Pressed`
    (set `self.HoldButton` true)
    (if (`self.HoldButton`) :!label _label_6
      (if (< _arrowmaxspeed 5000.0)
        (set `self.ArrowMaxSpeed` (+ _arrowmaxspeed 1000.0))
        (`KismetSystemLibrary.Delay` 0.05)
        (goto _label_6))))
  (:`Released`
    (set `self.HoldButton` false)
    (bind _returnvalue (`|SpawnActorFromClass` "/Game/Horse_Legacy/Blueprints/BP_ArrowFly.BP_ArrowFly_C" (`KismetMathLibrary.MakeTransform` (`SceneComponent.K2_GetComponentLocation` (`self.Sphere`)) (`KismetMathLibrary.MakeRotator` (.roll (`SceneComponent.K2_GetComponentRotation` (`self.Camera`))) (+ (.pitch (`SceneComponent.K2_GetComponentRotation` (`self.Camera`))) 15.0) (.yaw (`SceneComponent.K2_GetComponentRotation` (`self.Camera`))))) "AlwaysSpawn" "OverrideRootScale" null null))
    (bind _projectilemovement (`/Game/Horse_Legacy/Blueprints/BP_ArrowFly.ProjectileMovement` _returnvalue))
    (set `MovementComponent.Velocity` (* (`MovementComponent.Velocity` _projectilemovement) (`self.ArrowMaxSpeed`)) _projectilemovement)
    (set `self.ArrowMaxSpeed` 0.0)))

(fn `AreBothLegsTriggered`
  (returns (Result :type Boolean))
  (if (and (`self.IsRightLegTrigger`) (`self.IsLeftLegTrigger`))
    (return true)
    (else
      (return false))))

(fn `Get Current Acceleration`
  (returns (Acceleration :type "Float (double-precision)"))
  (return (`BlueprintMapLibrary.Map_Find` (`self.MoveStateAccelMap`) (`self.MovementState`))))

(fn `GetCurrentDuration`
  (returns (Duration :type "Float (double-precision)"))
  (return (`BlueprintMapLibrary.Map_Find` (`self.MoveStateDurationMap`) (`self.MovementState`))))

(fn `GetCurrentMaxSpeed`
  (returns (Value :type "Float (double-precision)"))
  (return (`BlueprintMapLibrary.Map_Find` (`self.MoveStateSpeedMap`) (`self.MovementState`))))

(fn `GetCurrentTurnSpeed`
  (returns (TurnSpeed :type "Float (double-precision)"))
  (return (`BlueprintMapLibrary.Map_Find` (`self.MoveStateTurnSpeedMap`) (`self.MovementState`))))

(fn `IncreaseMoveState`
  (switch `/Game/Horse_Legacy/Blueprints/ENUM_HorseMoveState` (`self.MovementState`)
    (:`NewEnumerator0`
      (bind _output_get (set `self.MovementState` (cast `/Game/Horse_Legacy/Blueprints/ENUM_HorseMoveState` (`KismetMathLibrary.BMin` (+ (`self.MovementState`) (`self.NbBothLegsTriggered`)) 3))))
      (`KismetSystemLibrary.PrintString` (`|GetEnumeratorNameAsString` _output_get))
      (`self.OnMoveStateChanged` (`self.MovementState`) :!label _label))
    (:`NewEnumerator1`
      (if (> (`self.NbBothLegsTriggered`) 1)
        (bind _output_get_2 (set `self.MovementState` (cast `/Game/Horse_Legacy/Blueprints/ENUM_HorseMoveState` (`KismetMathLibrary.BMin` (+ (- (`self.MovementState`) 1) (`self.NbBothLegsTriggered`)) 3))))
        (`KismetSystemLibrary.PrintString` (`|GetEnumeratorNameAsString` _output_get_2))
        (goto _label)))
    (:`NewEnumerator2`
      (if (> (`self.NbBothLegsTriggered`) 2)
        (bind _output_get_3 (set `self.MovementState` "NewEnumerator3"))
        (`KismetSystemLibrary.PrintString` (`|GetEnumeratorNameAsString` _output_get_3))
        (goto _label)))))

(fn `SetCurrentSpeed`
  (params (Amount :type "Float (double-precision)"))
  (bind _output_get (set `self.CurrentSpeed` Amount))
  (`self.OnCurrentSpeedChange` _output_get))

(fn `UpdateBothLegsTimer`
  (if (`self.IsSpecialMoving`)
    _
    (elif (not (`NavMovementComponent.IsFalling` (`self.CharacterMovement`)))
      ;[1 1 1] Start timer at first trigger LT + RT
      (if (> (`self.NbBothLegsTriggered`) 0)
        (if (`|EnumEquality` (`self.MovementState`) "NewEnumerator0")
          ;[1 1 1] Begin to move because player LT + RT atleast x1
          (set `self.MovementState` "NewEnumerator1")
          (`self.OnMoveStateChanged` (`self.MovementState`)))
        ;[1 1 1] Timer for inputs legs LT + RT
        (if (>= (`self.ElapsedTimeBothLegs`) (`self.TimeToIncreaseMoveState`))
          ;[1 1 1] Handle change of move state
          (if (> (`self.NbBothLegsTriggered`) 1)
            (if (< (`self.MovementState`) (enumliteral `/Game/Horse_Legacy/Blueprints/ENUM_HorseMoveState` "NewEnumerator3"))
              (`self.IncreaseMoveState`)
              (if (> (`self.NbBothLegsTriggered`) 3)
                (set `self.NbAccelerationBonus` (+ (`self.NbAccelerationBonus`) (`KismetMathLibrary.Conv_ByteToDouble` (- (`self.NbBothLegsTriggered`) 3)))))
              (elif (`self.IsAccelerating`)
                (set `self.NbAccelerationBonus` (+ (`self.NbAccelerationBonus`) (`KismetMathLibrary.Conv_ByteToDouble` (`self.NbBothLegsTriggered`))))
                (elif (> (`self.NbBothLegsTriggered`) 2)
                  (set `self.HasToRear` true))))
            (elif (and (`|EnumInequality` (`self.MovementState`) "NewEnumerator1") (`|EnumInequality` (`self.MovementState`) "NewEnumerator0"))
              (set `self.ElapsedStateDurationTime` 0.0)))
          ;;[1 1 1] Reset inputs and timer
          (set `self.NbBothLegsTriggered` 0)
          (set `self.ElapsedTimeBothLegs` 0.0)
          (else
            (bind _output_get (set `self.ElapsedTimeBothLegs` (+ (`self.DeltaTime`) (`self.ElapsedTimeBothLegs`))))))
        (else
          ;[1 1 1] Timer for movement duration (trot / gallop)
          (if (and (`|EnumInequality` (`self.MovementState`) "NewEnumerator1") (`|EnumInequality` (`self.MovementState`) "NewEnumerator0"))
            (bind _output_get_2 (set `self.ElapsedStateDurationTime` (+ (`self.ElapsedStateDurationTime`) (`self.DeltaTime`))))
            (if (>= _output_get_2 (`self.GetCurrentDuration`))
              (bind _output_get_3 (set `self.MovementState` (cast `/Game/Horse_Legacy/Blueprints/ENUM_HorseMoveState` (- (`self.MovementState`) 1))))
              (`self.OnMoveStateChanged` _output_get_3)
              (set `self.DecelerateSpeed` (/ (`self.CurrentSpeed`) (`self.DecelarateDelay`))))))))))

(fn `UserConstructionScript`)